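; BP_DamageBox is a hazard volume that hurts the third-person character while it stands inside.
; On BeginPlay it spawns a thunderstorm particle effect at its location.
; When BP_ThirdPersonCharacter begins overlapping the DamageBox component, it caches the character and starts a looping timer that repeatedly applies fixed damage.
; End overlap clears that timer through the stored handle.
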(event OnComponentBeginOverlap(DamageBox)
  (params (OverlappedComponent :type Primitive%20Component%20Object%20Reference) (OtherActor :type Actor%20Object%20Reference) (OtherComp :type Primitive%20Component%20Object%20Reference) (OtherBodyIndex :type Integer) (bFromSweep :type Boolean) (SweepResult :type Hit%20Result%20Structure%20%28by%20ref%29))
  ;[1 1 1] Damage box collision event
  (bind _asbp_third_person_character (Utilities|Casting|CastToBP_ThirdPersonCharacter OtherActor))
  (Variables|Default|SetAs%20BP%20Third%20Person%20Character _asbp_third_person_character)
  (bind _returnvalue (Utilities|Time|SetTimerbyEvent (delegate Custom|DamagePlayer) 0.3 true))
  (Variables|Default|SetTimerRef _returnvalue))

(event OnComponentEndOverlap(DamageBox)
  (params (OverlappedComponent :type Primitive%20Component%20Object%20Reference) (OtherActor :type Actor%20Object%20Reference) (OtherComp :type Primitive%20Component%20Object%20Reference) (OtherBodyIndex :type Integer))
  ;[1 1 1] Damage box collision event
  (Utilities|Casting|CastToBP_ThirdPersonCharacter OtherActor)
  (Utilities|Time|ClearandInvalidateTimerbyHandle (Variables|Default|GetTimerRef)))

(event Custom|DamagePlayer
  ;[1 1 1] Damage box collision event
  (Game|Damage|ApplyDamage (Variables|Default|GetAs%20BP%20Third%20Person%20Character) 1e+01 0 0))

(event EventBeginPlay
  (Effects|SpawnEmitteratLocation "/Game/FXVarietyPack/Particles/P_ky_thunderStorm.P_ky_thunderStorm" (Transformation|GetActorLocation)))

(fn ConstructionScript)